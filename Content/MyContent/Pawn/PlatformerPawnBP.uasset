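; Platformer player pawn that creates its PlayerUI on BeginPlay, caps floating movement speed and handles camera pitch and the pause menu.
; Each Tick it sets OnGround from whether the Box overlaps any actor, and prints it as debug output.
; LookUp input pitches the SpringArm, while Escape opens PauseMenu with cursor and UI input without pausing the game.
; HideUI removes the widget from the viewport, but ShowUI only restores visibility.
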(event OnComponentBeginOverlap(Box)
  (params (OverlappedComponent :type Primitive%20Component%20Object%20Reference) (OtherActor :type Actor%20Object%20Reference) (OtherComp :type Primitive%20Component%20Object%20Reference) (OtherBodyIndex :type Integer) (bFromSweep :type Boolean) (SweepResult :type Hit%20Result%20Structure%20%28by%20ref%29)))

(event OnComponentEndOverlap(Box)
  (params (OverlappedComponent :type Primitive%20Component%20Object%20Reference) (OtherActor :type Actor%20Object%20Reference) (OtherComp :type Primitive%20Component%20Object%20Reference) (OtherBodyIndex :type Integer)))

(event EventBeginPlay
  (bind _returnvalue (UserInterface|CreateWidget "/Game/MyContent/Ui/PlayerUI.PlayerUI_C"))
  (Variables|/Game/MyContent/Ui/PlayerUI.PlayerUI_C|Setplayer _returnvalue self)
  (Variables|Default|SetUIWidget _returnvalue)
  (UserInterface|Viewport|AddtoViewport _returnvalue 0)
  (Variables|/Script/Engine.FloatingPawnMovement|SetMaxSpeed (Variables|Default|GetFloatingPawnMovement) 5e+02))

(event Collision|EventActorBeginOverlap
  (params (OtherActor :type Actor%20Object%20Reference)))

(event EventTick
  (params (DeltaSeconds :type Float%20%28single-precision%29))
  (if (== (Utilities|Array|Length (Collision|GetOverlappingActors (Variables|Default|GetBox) 0 :!class /Script/Engine.PrimitiveComponent)) 0)
    (Variables|Default|SetonGround false)
    (else
      (Variables|Default|SetonGround true)))
  (Development|PrintString (Utilities|String|ToString(Boolean) (Variables|Default|GetonGround))))

(event Input|ActionEvents|InputActionEscape
  (params (Key :type Key%20Structure :default "None"))
  (:Pressed
    (bind _returnvalue (UserInterface|CreateWidget "/Game/MyContent/Ui/PauseMenu.PauseMenu_C"))
    (UserInterface|Viewport|AddtoViewport _returnvalue 0)
    (Input|SetInputModeGameandUI 0 _returnvalue "LockAlways" false false)
    (Variables|/Script/Engine.PlayerController|SetbShowMouseCursor (Game|GetPlayerController 0) true)))

(event Input|AxisEvents|InputAxisLookUp
  (params (AxisValue :type Float%20%28single-precision%29))
  (bind _springarm (Variables|Default|GetSpringArm))
  (bind _returnvalue (Transformation|GetWorldRotation _springarm))
  (Transformation|SetWorldRotation (Variables|Default|GetSpringArm) (Math|Rotator|MakeRotator (.roll _returnvalue) (+ AxisValue (.pitch _returnvalue)) (.yaw _returnvalue)) false false))

(fn ConstructionScript)

(fn ShowUI
  (Variables|/Script/UMG.Widget|SetVisibility (Variables|Default|GetUIWidget) "Visible"))

(fn HideUI
  (bind _uiwidget (Variables|Default|GetUIWidget))
  (Variables|/Script/UMG.Widget|SetVisibility _uiwidget "Hidden")
  (Widget|RemovefromParent _uiwidget))