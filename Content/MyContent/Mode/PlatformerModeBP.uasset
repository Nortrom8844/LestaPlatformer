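; Game mode for a platformer that sets input mode and presents the victory and defeat end screens.
; At begin play and on game start it switches to game-only input if the player pawn is a PlatformerPawnBP.
; Victory and defeat events each create their widget and play a sound.
; A shared function shows the widget with Game and UI input and mouse cursor, then hides the pawn's UI.
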(event EventBeginPlay
  (Utilities|Casting|CastToPlatformerPawnBP (Game|Player|GetPlayerPawn 0)
    (:then
      (Input|SetInputModeGameOnly (Game|GetPlayerController 0) false))
    (:CastFailed
      (Development|PrintString "Pawn cast failed"))))

(event EventTick
  (params (DeltaSeconds :type Float%20%28single-precision%29)))

(event EventOnVictory
  (bind _returnvalue (UserInterface|CreateWidget "/Game/MyContent/Ui/VictoryScreen.VictoryScreen_C"))
  (CallFunction|ShowEndGameScreen _returnvalue)
  (Audio|PlaySound2D "/Game/Interface_And_Item_Sounds/Cues/Special_Powerup_01_Cue.Special_Powerup_01_Cue" 1.0 1.0 0.0 0 0))

(event EventOnDefeat
  (bind _returnvalue (UserInterface|CreateWidget "/Game/MyContent/Ui/DefeatScreen.DefeatScreen_C"))
  (CallFunction|ShowEndGameScreen _returnvalue)
  (Audio|PlaySound2D "/Game/Interface_And_Item_Sounds/Cues/Discordant_GameOver_Musical_Short_Cue.Discordant_GameOver_Musical_Short_Cue" 1.0 1.0 0.0 0 0))

(event EventOnStartGame
  (Utilities|Casting|CastToPlatformerPawnBP (Game|Player|GetPlayerPawn 0)
    (:then
      (Input|SetInputModeGameOnly (Game|GetPlayerController 0) false))
    (:CastFailed
      (Development|PrintString "Pawn cast failed"))))

(fn ConstructionScript)

(fn ShowEndGameScreen
  (params (NewParam :type User%20Widget%20Object%20Reference))
  (bind _returnvalue (Game|GetPlayerController 0))
  (UserInterface|Viewport|AddtoViewport NewParam 0)
  (Input|SetInputModeGameandUI _returnvalue NewParam "DoNotLock" false false)
  (Variables|/Script/Engine.PlayerController|SetbShowMouseCursor _returnvalue true)
  (bind _asplatformer_pawn_bp (Utilities|Casting|CastToPlatformerPawnBP (Game|Player|GetPlayerPawn 0)))
  (Default|HideUI _asplatformer_pawn_bp))