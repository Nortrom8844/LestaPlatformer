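; Platform that arms when the player pawn stands on it, then explodes and damages whoever is still on it.
; Tick polls the Box for PlatformerPawnBP overlaps and, when IsReady, calls StartTimer, swaps the mesh to orange and plays a switch sound.
; OnExplode restores the saved material, then applies GetDamage to each overlapping pawn with an explosion sound.
; Readiness, timer and damage value come from functions defined outside this graph.
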(event EventBeginPlay)

(event Collision|EventActorBeginOverlap
  (params (OtherActor :type Actor%20Object%20Reference)))

(event EventTick
  (params (DeltaSeconds :type Float%20%28single-precision%29))
  (bind _mesh (Variables|Character|GetMesh))
  (if (> (Utilities|Array|Length (Collision|GetOverlappingActors (Variables|Default|GetBox) "/Game/MyContent/Pawn/PlatformerPawnBP.PlatformerPawnBP_C" :!class /Script/Engine.PrimitiveComponent)) 0)
    (bind _returnvalue (Class|ExplosionPlatform|IsReady))
    (if _returnvalue
      (Class|ExplosionPlatform|StartTimer)
      (Variables|Default|SetDefaultMaterial (Rendering|Material|GetMaterial _mesh 0))
      (Rendering|Material|SetMaterial _mesh 0 "/Game/MyContent/Platforms/Materials/Orange.Orange")
      (Audio|PlaySound2D "/Game/Interface_And_Item_Sounds/Cues/Flick_Switch_05_Cue.Flick_Switch_05_Cue" 1.0 1.0 0.0 0 0))))

(event EventOnExplode
  (Rendering|Material|SetMaterial (Variables|Character|GetMesh) 0 (Variables|Default|GetDefaultMaterial))
  (for _array_element (Collision|GetOverlappingActors (Variables|Default|GetBox) "/Game/MyContent/Pawn/PlatformerPawnBP.PlatformerPawnBP_C" :!class /Script/Engine.PrimitiveComponent)
    (bind _asplatformer_pawn_bp (Utilities|Casting|CastToPlatformerPawnBP _array_element))
    (bind _returnvalue (Class|ExplosionPlatform|GetDamage))
    (Class|PlatformerPawn|TakeDamage _asplatformer_pawn_bp _returnvalue)
    (Audio|PlaySound2D "/Game/Interface_And_Item_Sounds/Explosion.Explosion" 1.0 1.0 0.0 0 0)))

(fn ConstructionScript)