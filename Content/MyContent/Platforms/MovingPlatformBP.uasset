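; Moving platform Blueprint that carries platformer pawns along with it.
; On BeginPlay, the world locations of two sphere components set the platform's start and end positions.
; The MovePawns event offsets each PlatformerPawnBP overlapping the Box component by the supplied move vector, without sweeping.
; The graph does not move the platform itself or call MovePawns.
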(event EventBeginPlay
  (Class|MovingPlatform|SetStartPosition (Transformation|GetWorldLocation (Variables|Default|GetSphere)))
  (Class|MovingPlatform|SetEndPosition (Transformation|GetWorldLocation (Variables|Default|GetSphere1))))

(event Collision|EventActorBeginOverlap
  (params (OtherActor :type Actor%20Object%20Reference)))

(event EventTick
  (params (DeltaSeconds :type Float%20%28single-precision%29)))

(event EventMovePawns
  (params (move :type Vector :default "0, 0, 0"))
  (for _array_element (Collision|GetOverlappingActors (Variables|Default|GetBox) "/Game/MyContent/Pawn/PlatformerPawnBP.PlatformerPawnBP_C" :!class /Script/Engine.PrimitiveComponent)
    (Transformation|SetActorLocation _array_element (+ (Transformation|GetActorLocation _array_element) move) false false)))

(fn ConstructionScript)