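; FakePlatformBP is a platform actor that can switch between a solid state and a non-collidable one.
; On BeginPlay it caches the mesh's original material.
; The Disappear event turns off collision, applies an alternate material and plays a 2D switch sound, while Appear restores collision and the cached material.
; Nothing in the Blueprint calls either event, so switching depends on external triggers.
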(event EventBeginPlay
  (Variables|Default|SetDefault%20material (Rendering|Material|GetMaterial (Variables|Character|GetMesh) 0)))

(event Collision|EventActorBeginOverlap
  (params (OtherActor :type Actor%20Object%20Reference)))

(event EventTick
  (params (DeltaSeconds :type Float%20%28single-precision%29)))

(event EventDisappear
  (bind _mesh (Variables|Character|GetMesh))
  (Collision|SetCollisionEnabled _mesh "NoCollision")
  (Rendering|Material|SetMaterial _mesh 0 (Variables|Default|GetMaterial))
  (Audio|PlaySound2D "/Game/Interface_And_Item_Sounds/Cues/Flick_Switch_05_Cue.Flick_Switch_05_Cue" 1.0 1.0 0.0 0 0))

(event EventAppear
  (bind _mesh (Variables|Character|GetMesh))
  (Collision|SetCollisionEnabled _mesh "QueryAndPhysics")
  (Rendering|Material|SetMaterial _mesh 0 (Variables|Default|GetDefault%20material)))

(fn ConstructionScript)